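; BP_MusicGate is a trigger volume that switches background music when the first-person character leaves its box.
; Each exit flips between NewSong and PreviousSong through a FlipFlop, so the choice follows crossing count rather than direction.
; The audio component fades out, waits out the fade with a Delay, then swaps the sound and fades back in.
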(event `self.Box.OnComponentEndOverlap`
  (params (OverlappedComponent :type "PrimitiveComponent Object Reference") (OtherActor :type "Actor Object Reference") (OtherComp :type "PrimitiveComponent Object Reference") (OtherBodyIndex :type Integer))
  (cast `/Game/FirstPerson/Blueprints/BP_FirstPersonCharacter` OtherActor)
  (`/Engine/EditorBlueprintResources/StandardMacros.FlipFlop`
    (:`A`
      (set `self.SwitchSong` (`self.NewSong`)))
    (:`B`
      (set `self.SwitchSong` (`self.PreviousSong`))))
  (`AudioComponent.FadeOut` (`self.Audio`) 1.5 0.0 "Linear")
  (`KismetSystemLibrary.Delay` 1.5)
  (`AudioComponent.SetSound` (`self.Audio`) (`self.SwitchSong`))
  (`AudioComponent.FadeIn` (`self.Audio`) 1.5 1.0 0.0 "Linear"))

(fn `UserConstructionScript`)