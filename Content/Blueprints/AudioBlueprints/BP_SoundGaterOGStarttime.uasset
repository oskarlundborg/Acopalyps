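; BP_SoundGaterOGStarttime is an audio gate that crossfades between two sets of placed sounds as the first-person character passes through it.
; Each time the character leaves BoxTrigger, a FlipFlop alternates between fading in Sounds2 while fading out Sounds1, and the reverse, over a shared fade duration.
; The fade-out loop is nested inside the fade-in loop, so it repeats for every sound faded in.
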(event `self.BoxTrigger.OnComponentEndOverlap`
  (params (OverlappedComponent :type "PrimitiveComponent Object Reference") (OtherActor :type "Actor Object Reference") (OtherComp :type "PrimitiveComponent Object Reference") (OtherBodyIndex :type Integer))
  (bind _sounds1 (`self.Sounds1`))
  (bind _fade_duration__overall_ (`self.Fade Duration (Overall)`))
  (bind _sounds2 (`self.Sounds2`))
  (cast `/Game/FirstPerson/Blueprints/BP_FirstPersonCharacter` OtherActor)
  (`/Engine/EditorBlueprintResources/StandardMacros.FlipFlop`
    (:`A`
      (for _array_element _sounds2
        (`AudioComponent.FadeIn` (`AmbientSound.AudioComponent` _array_element) _fade_duration__overall_ 1.0 0.0 "Linear")
        (for _array_element_2 _sounds1
          (`AudioComponent.FadeOut` (`AmbientSound.AudioComponent` _array_element_2) _fade_duration__overall_ 0.0 "Linear"))))
    (:`B`
      (for _array_element_3 _sounds1
        (`AudioComponent.FadeIn` (`AmbientSound.AudioComponent` _array_element_3) _fade_duration__overall_ 1.0 0.0 "Linear")
        (for _array_element_4 _sounds2
          (`AudioComponent.FadeOut` (`AmbientSound.AudioComponent` _array_element_4) _fade_duration__overall_ 0.0 "Linear"))))))

(fn `UserConstructionScript`)