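; BP_CombatTrigger is a one-shot trigger that starts combat when the player's BP_FirstPersonCharacter overlaps it.
; If NewMissionToSet is non-empty, it updates the character's mission and plays TriggerSoundClip as a 2D sound.
; It then calls StartCombat, prints a debug message and sets TriggerUsed so later overlaps do nothing.
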(event `self.ReceiveActorBeginOverlap`
  (params (OtherActor :type "Actor Object Reference"))
  (bind _newmissiontoset (`self.NewMissionToSet`))
  (bind _asbp_first_person_character (cast `/Game/FirstPerson/Blueprints/BP_FirstPersonCharacter` OtherActor))
  (if (not (`self.bTriggerUsed`))
    (switch `int` (`KismetStringLibrary.Len` _newmissiontoset)
      (:`Default`
        (`/Game/FirstPerson/Blueprints/BP_FirstPersonCharacter.UpdateMission` _asbp_first_person_character _newmissiontoset)
        (`GameplayStatics.PlaySound2D` (`self.TriggerSoundClip`) 1.0 1.0 0.0 null null))
      (:`0`
        _))
    (`self.StartCombat`)
    (`KismetSystemLibrary.PrintString` "Combat Started")
    (set `self.bTriggerUsed` true)))

(fn `UserConstructionScript`)