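; BP_CombatManager handles the start and end of a combat encounter, with music, mission updates and an optional gate.
; BeginPlay destroys the Gate component when HasGate is off.
; StartOfCombat plays combat music and shows an artist and song popup.
; When FinalManager is set, EndOfCombat plays closing sounds and updates the player's mission once; a failed player cast routes to the gate removal instead.
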(event `self.ReceiveBeginPlay`
  (bind _gate (`self.Gate`))
  (if (not (`self.bHasGate`))
    (`/Engine/EditorBlueprintResources/StandardMacros.IsValid` _gate :!label _label
      (:`Is Valid`
        (`ActorComponent.K2_DestroyComponent` _gate)))))

(event `self.StartOfCombat`
  (`GameplayStatics.PlaySound2D` (`self.CombatMusic`) 1.0 1.0 0.0 null null)
  (bind _returnvalue (`|CreateWidget` "/Game/UserInterface/PopupMusicText.PopupMusicText_C"))
  (set `/Game/UserInterface/PopupMusicText.CurrentArtistName` (`self.Current Artist Name`) _returnvalue)
  (set `/Game/UserInterface/PopupMusicText.CurrentSongName` (`self.Current Song Name`) _returnvalue)
  (`UserWidget.AddToViewport` _returnvalue 0))

(event `self.EndOfCombat`
  (bind _endofcombatmissionstring (`self.EndOfCombatMissionString`))
  (bind _asbp_first_person_character (cast `/Game/FirstPerson/Blueprints/BP_FirstPersonCharacter` (`GameplayStatics.GetPlayerCharacter` 0))
    (:`then`
      (if (`self.bFinalManager`)
        (`GameplayStatics.PlaySound2D` "/Game/Audio/OST/Silent_Placeholder.Silent_Placeholder" 1.0 1.0 0.0 null null)
        (`GameplayStatics.PlaySound2D` (`self.EndOfCombatSoundClip`) 1.0 1.0 0.0 null null)
        (`/Engine/EditorBlueprintResources/StandardMacros.DoOnce` false
          (:`Completed`
            (switch `int` (`KismetStringLibrary.Len` _endofcombatmissionstring)
              (:`Default`
                (`/Game/FirstPerson/Blueprints/BP_FirstPersonCharacter.UpdateMission` _asbp_first_person_character _endofcombatmissionstring)))))))
    (:`CastFailed`
      (goto _label))))

(fn `UserConstructionScript`)