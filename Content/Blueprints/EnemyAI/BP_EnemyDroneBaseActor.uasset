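; Base enemy drone Blueprint that adds audio, death effects and loot to the drone's attack and death events.
; Attack events play attached cues, while a randomly offset rotor loop takes its pitch parameter from CurrentSpeed each tick.
; On death it stops the rotor, plays death sounds and triggers delayed explosion and staggered fire effects.
; It also has a roughly two-in-three chance to spawn an ammo box where a downward trace hits.
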(event `self.OnPrepareForAttackEvent`
  (bind _dronemesh (`self.DroneMesh`))
  (`GameplayStatics.SpawnSoundAttached` "/Game/Audio/SFX/Combat/Enemy/Drone/Drone_PrepareAttackCue.Drone_PrepareAttackCue" _dronemesh "None" (0.0 0.0 0.0) (struct) "KeepRelativeOffset" false 1.0 1.0 0.0 null null)
  (`GameplayStatics.SpawnSoundAttached` "/Game/Audio/SFX/Combat/Enemy/Drone/VoiceLines/DroneCombatLiners.DroneCombatLiners" _dronemesh "None" (0.0 0.0 0.0) (struct) "KeepRelativeOffset" false 1.0 1.0 0.0 null null))

(event `self.OnAttackEvent`
  (`GameplayStatics.SpawnSoundAttached` "/Game/Audio/SFX/Combat/Enemy/Drone/Drone_AttackCue.Drone_AttackCue" (`self.DroneMesh`) "None" (0.0 0.0 0.0) (struct) "KeepRelativeOffset" false 1.0 1.0 0.0 null null))

(event `self.ReceiveHit`
  (params (MyComp :type "PrimitiveComponent Object Reference") (Other :type "Actor Object Reference") (OtherComp :type "PrimitiveComponent Object Reference") (bSelfMoved :type Boolean) (HitLocation :type "Vector Structure") (HitNormal :type "Vector Structure") (NormalImpulse :type "Vector Structure") (Hit :type "HitResult Structure (by ref)")))

(event `self.OnDeathEvent`
  (bind _returnvalue (`self.K2_GetActorLocation`))
  (bind _burning (`self.Burning`))
  (bind _burning2 (`self.Burning2`))
  (bind _burning1 (`self.Burning1`))
  (bind _explosion (`self.Explosion`))
  ;[1 1 1] OnDeath Ammo/Health Drop
  (`|ExecutionSequence`
    (:`then_0`
      (`KismetSystemLibrary.Delay` 1.2)
      (`SceneComponent.SetVisibility` _explosion true false)
      (`NiagaraFunctionLibrary.SpawnSystemAtLocation` (`NiagaraComponent.GetAsset` _explosion) (`SceneComponent.K2_GetComponentLocation` _explosion))
      (`GameplayStatics.PlaySound2D` "/Game/Audio/SFX/Combat/Grenades__Redacted_/Explosive/S_Explosion_2.S_Explosion_2" 1.0 1.0 0.0 null null)
      (`|ExecutionSequence`
        (:`then_0`
          (`KismetSystemLibrary.Delay` 0.3)
          (`SceneComponent.SetVisibility` _burning true false)
          (bind _returnvalue_2 (`NiagaraFunctionLibrary.SpawnSystemAtLocation` (`NiagaraComponent.GetAsset` _burning) (`SceneComponent.K2_GetComponentLocation` _burning)))
          (`KismetSystemLibrary.Delay` 5.0)
          (`ActorComponent.K2_DestroyComponent` _returnvalue_2))
        (:`then_1`
          (`KismetSystemLibrary.Delay` 0.2)
          (`SceneComponent.SetVisibility` _burning2 true false)
          (bind _returnvalue_3 (`NiagaraFunctionLibrary.SpawnSystemAtLocation` (`NiagaraComponent.GetAsset` _burning2) (`SceneComponent.K2_GetComponentLocation` _burning2)))
          (`KismetSystemLibrary.Delay` 5.0)
          (`ActorComponent.K2_DestroyComponent` _returnvalue_3))
        (:`then_2`
          (`KismetSystemLibrary.Delay` 0.4)
          (`SceneComponent.SetVisibility` _burning1 true false)
          (bind _returnvalue_4 (`NiagaraFunctionLibrary.SpawnSystemAtLocation` (`NiagaraComponent.GetAsset` _burning1) (`SceneComponent.K2_GetComponentLocation` _burning1)))
          (`KismetSystemLibrary.Delay` 5.0)
          (`ActorComponent.K2_DestroyComponent` _returnvalue_4))))
    (:`then_1`
      (`GameplayStatics.SpawnSoundAttached` "/Game/Audio/SFX/Combat/Enemy/Drone/VoiceLines/DroneDeathCue.DroneDeathCue" (`self.DroneMesh`) "None" (0.0 0.0 0.0) (struct) "KeepRelativeOffset" false 1.0 1.0 0.0 null null)
      (`AudioComponent.Stop` (`self.Drone_RotorsCue`))
      (if (> (`KismetMathLibrary.RandomIntegerInRange` 0 100) 33)
        (bind (_outhit _returnvalue_5) (`KismetSystemLibrary.LineTraceSingle` _returnvalue (+ _returnvalue (* (`KismetMathLibrary.Vector_Down`) (1000.0 1000.0 1000.0))) "TraceTypeQuery1"))
        (if _returnvalue_5
          (`|SpawnActorFromClass` "/Game/Blueprints/EnemyDrops/BP_Ammobox.BP_Ammobox_C" (`KismetMathLibrary.Conv_VectorToTransform` (`.ImpactPoint` (`GameplayStatics.BreakHitResult` _outhit))) "AdjustIfPossibleButAlwaysSpawn" "OverrideRootScale" null null))))))

(event `self.ReceiveTick`
  (params (DeltaSeconds :type "Float (single-precision)"))
  ;[1 1 1] OnDeath Ammo/Health Drop
  (`AudioParameterControllerInterface.SetFloatParameter` (`self.Drone_RotorsCue`) "RotorPitch" (`self.CurrentSpeed`)))

(event `self.ReceiveBeginPlay`
  (bind _drone_rotorscue (`self.Drone_RotorsCue`))
  ;[1 1 1] OnDeath Ammo/Health Drop
  (`AudioComponent.Play` _drone_rotorscue (`KismetMathLibrary.RandomFloatInRange` 0.0 (`SoundBase.Duration` (`AudioComponent.Sound` _drone_rotorscue)))))

(fn `UserConstructionScript`)