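; BP_EnemyGun is a gun Blueprint that supplies audiovisual feedback for weapon events, presumably inherited from a parent class.
; Firing spawns a muzzle flash and a sound chosen by ammo type; empty-magazine attempts and Explosive or Flare readiness play cues.
; Despite the enemy name, reloading plays a montage on player 0's first-person arms, animates the gun and adds a reloading HUD widget.
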(event `self.OnCanFire`
  (params (AmmoType :type "AMMO_TYPES Enum" :default "Regular"))
  ;[1 1 1] Ready Secondary Sound
  (switch `AMMO_TYPES` AmmoType
    (:`Explosive`
      _)
    (:`Flare`
      _))
  (`GameplayStatics.SpawnSoundAttached` "/Game/Audio/SFX/Player/Weapon/Management/S_SecondaryReadyCue.S_SecondaryReadyCue" (`self.SkeletalMesh`) "None" (0.0 0.0 0.0) (struct) "KeepRelativeOffset" false 1.0 1.0 0.0 null null))

(event `self.ReloadTriggerEvent`
  ;[1 1 1] Play Reload Animation
  (`|PlayMontage` (`AcopalypsCharacter.Mesh1P` (cast `/Game/FirstPerson/Blueprints/BP_FirstPersonCharacter` (`GameplayStatics.GetPlayerCharacter` 0) :!pure true)) "/Game/FirstPersonArms/Animations/FP_Reload_Montage.FP_Reload_Montage"
    (:`then`
      (`SkeletalMeshComponent.PlayAnimation` (`self.SkeletalMesh`) "/Game/FirstPersonArms/Animations/A_Gun_Reload.A_Gun_Reload" false)
      ;[1 1 1] HUD Reload
      (`GameplayStatics.SpawnSound2D` null 1.0 1.0 0.0 null)
      (bind _returnvalue (`|CreateWidget` "/Game/UserInterface/W_Reloading.W_Reloading_C"))
      (`UserWidget.AddToViewport` _returnvalue 0))))

(event `self.EmptyMagFireAttemptEvent`
  ;[1 1 1] Skjutljud
  (`GameplayStatics.SpawnSoundAttached` "/Game/Audio/SFX/Player/Weapon/Management/Switch/EmptyMagCue.EmptyMagCue" (`self.SkeletalMesh`) "None" (0.0 0.0 0.0) (struct) "KeepRelativeOffset" false 1.0 1.0 0.0 null null))

(event `self.FireTriggerEvent`
  (params (Hit :type "HitResult Structure (by ref)") (ShotDirection :type "Vector Structure (by ref)") (AmmoType :type "AMMO_TYPES Enum" :default "Regular"))
  (bind _skeletalmesh (`self.SkeletalMesh`))
  (`|ExecutionSequence`
    (:`then_0`
      ;[1 1 1] Spawn MuzzleFlash Regular
      (`NiagaraFunctionLibrary.SpawnSystemAttached` (`self.MuzzleFlash`) (`self.SkeletalMesh`) "Muzzle" (0.0 0.0 0.0) (struct :`Yaw` -90.0) "SnapToTarget"))
    (:`then_2`
      ;[1 1 1] Skjutljud
      (switch `AMMO_TYPES` AmmoType
        (:`Regular`
          (`GameplayStatics.SpawnSoundAttached` "/Game/Audio/SFX/Player/Weapon/Default/ShootDefaultLayered.ShootDefaultLayered" _skeletalmesh "None" (0.0 0.0 0.0) (struct) "KeepRelativeOffset" false 1.0 1.0 0.0 null null))
        (:`Bouncing`
          (`GameplayStatics.SpawnSoundAttached` "/Game/Audio/SFX/Player/Weapon/Default/ShootDefaultLayered.ShootDefaultLayered" _skeletalmesh "None" (0.0 0.0 0.0) (struct) "KeepRelativeOffset" false 1.0 1.0 0.0 null null))
        (:`Explosive`
          (`GameplayStatics.SpawnSoundAttached` "/Game/Audio/SFX/Player/Weapon/Explosive/S_RocketLaunch.S_RocketLaunch" _skeletalmesh "None" (0.0 0.0 0.0) (struct) "KeepRelativeOffset" false 1.0 1.0 0.0 null null))
        (:`Flare`
          (`GameplayStatics.SpawnSoundAttached` "/Game/Audio/SFX/Player/Weapon/Explosive/S_RocketLaunch.S_RocketLaunch" _skeletalmesh "None" (0.0 0.0 0.0) (struct) "KeepRelativeOffset" false 1.0 1.0 0.0 null null))
        (:`Rapid`
          (`GameplayStatics.SpawnSoundAttached` "/Game/Audio/SFX/Player/Weapon/Default/ShootDefaultLayered.ShootDefaultLayered" _skeletalmesh "None" (0.0 0.0 0.0) (struct) "KeepRelativeOffset" false 1.0 1.0 0.0 null null))
        (:`Shotgun`
          (`GameplayStatics.SpawnSoundAttached` "/Game/Audio/SFX/Player/Weapon/Shotgun/ShotgunFireCue.ShotgunFireCue" _skeletalmesh "None" (0.0 0.0 0.0) (struct) "KeepRelativeOffset" false 1.0 1.0 0.0 null null))))))

(fn `UserConstructionScript`)