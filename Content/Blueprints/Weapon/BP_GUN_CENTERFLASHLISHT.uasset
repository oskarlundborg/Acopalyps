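; Gun Blueprint that adds sound, muzzle flash and HUD feedback to weapon events, plus a flashlight that follows the crosshair.
; Fire events spawn the muzzle flash and a sound chosen by ammo type; Explosive and Flare also get a ready cue.
; Reload and empty-magazine events play sounds and manage the Reloading and No Ammo widgets.
; Each tick, a hit trace steers the flashlight toward the impact point using smoothed rotation.
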(event `self.OnCanFire`
  (params (AmmoType :type "AMMO_TYPES Enum" :default "Regular"))
  ;[1 1 1] Ready Secondary Sound
  (switch `AMMO_TYPES` AmmoType
    (:`Explosive`
      _)
    (:`Flare`
      _))
  (`GameplayStatics.SpawnSoundAttached` "/Game/Audio/SFX/Player/Weapon/Management/S_SecondaryReadyCue.S_SecondaryReadyCue" (`self.SkeletalMesh`) "None" (0.0 0.0 0.0) (struct) "KeepRelativeOffset" false 1.0 1.0 0.0 null null))

(event `self.ReloadCompletedEvent`
  ;[1 1 1] Event Reload Complete
  (`|ExecutionSequence`
    (:`then_0`
      (if (`self.bNoAmmo`)
        (`Widget.RemoveFromParent` (stale `self.FireTriggerEvent` _returnvalue))
        (set `self.bNoAmmo` false)))
    (:`then_1`
      (`Widget.RemoveFromParent` (stale `self.ReloadTriggerEvent` _returnvalue)))))

(event `self.ReloadTriggerEvent`
  ;[1 1 1] Skjutljud
  (`GameplayStatics.SpawnSound2D` "/Game/Audio/SFX/Player/Weapon/Management/ReloadingSoundCue.ReloadingSoundCue" 1.0 1.0 0.0 null)
  ;[1 1 1] HUD Reload
  (bind _returnvalue (`|CreateWidget` "/Game/UserInterface/W_Reloading.W_Reloading_C"))
  (`UserWidget.AddToViewport` _returnvalue 0))

(event `self.EmptyMagFireAttemptEvent`
  ;[1 1 1] Skjutljud
  (`GameplayStatics.SpawnSoundAttached` "/Game/Audio/SFX/Player/Weapon/Management/Switch/EmptyMagCue.EmptyMagCue" (`self.SkeletalMesh`) "None" (0.0 0.0 0.0) (struct) "KeepRelativeOffset" false 1.0 1.0 0.0 null null))

(event `self.FireTriggerEvent`
  (params (Hit :type "HitResult Structure (by ref)") (ShotDirection :type "Vector Structure (by ref)") (AmmoType :type "AMMO_TYPES Enum" :default "Regular"))
  (bind _skeletalmesh (`self.SkeletalMesh`))
  (`|ExecutionSequence`
    (:`then_0`
      ;[1 1 1] Spawn MuzzleFlash Regular
      (`NiagaraFunctionLibrary.SpawnSystemAttached` (`self.MuzzleFlash`) (`self.SkeletalMesh`) "Muzzle" (0.0 0.0 0.0) (struct) "KeepRelativeOffset"))
    (:`then_1`
      ;[1 1 1] HUD No Ammo
      (if (<= (`self.CurrentMag`) 0)
        (bind _returnvalue (`|CreateWidget` "/Game/UserInterface/W_NoAmmo.W_NoAmmo_C"))
        (`UserWidget.AddToViewport` _returnvalue 0)
        (set `self.bNoAmmo` true)))
    (:`then_2`
      ;[1 1 1] Skjutljud
      (switch `AMMO_TYPES` AmmoType
        (:`Regular`
          (`GameplayStatics.SpawnSoundAttached` "/Game/Audio/SFX/Player/Weapon/Default/ShootDefaultLayered.ShootDefaultLayered" _skeletalmesh "None" (0.0 0.0 0.0) (struct) "KeepRelativeOffset" false 1.0 1.0 0.0 null null))
        (:`Bouncing`
          (`GameplayStatics.SpawnSoundAttached` "/Game/Audio/SFX/Player/Weapon/Default/ShootDefaultLayered.ShootDefaultLayered" _skeletalmesh "None" (0.0 0.0 0.0) (struct) "KeepRelativeOffset" false 1.0 1.0 0.0 null null))
        (:`Explosive`
          (`GameplayStatics.SpawnSoundAttached` "/Game/Audio/SFX/Player/Weapon/Explosive/S_Flare_Launcher_SPM.S_Flare_Launcher_SPM" _skeletalmesh "None" (0.0 0.0 0.0) (struct) "KeepRelativeOffset" false 1.0 1.0 0.0 null null))
        (:`Flare`
          (`GameplayStatics.SpawnSoundAttached` "/Game/Audio/SFX/Player/Weapon/Explosive/S_Flare_Launcher_SPM.S_Flare_Launcher_SPM" _skeletalmesh "None" (0.0 0.0 0.0) (struct) "KeepRelativeOffset" false 1.0 1.0 0.0 null null))
        (:`Rapid`
          (`GameplayStatics.SpawnSoundAttached` "/Game/Audio/SFX/Player/Weapon/Default/ShootRapidLayered.ShootRapidLayered" _skeletalmesh "None" (0.0 0.0 0.0) (struct) "KeepRelativeOffset" false 1.0 1.0 0.0 null null))
        (:`Shotgun`
          (`GameplayStatics.SpawnSoundAttached` "/Game/Audio/SFX/Player/Weapon/Shotgun/ShotgunFireCue.ShotgunFireCue" _skeletalmesh "None" (0.0 0.0 0.0) (struct) "KeepRelativeOffset" false 1.0 1.0 0.0 null null))))))

(event `self.ReceiveTick`
  (params (DeltaSeconds :type "Float (single-precision)"))
  (bind _flashlight (`self.Flashlight`))
  (bind _returnvalue (`SceneComponent.K2_GetComponentRotation` _flashlight))
  ;[1 1 1] Rotate Flashlight Towards Crosshair
  (bind (_hit _shotdirection _returnvalue_2) (`self.HitTrace`))
  (if _returnvalue_2
    (`SceneComponent.K2_SetWorldRotation` _flashlight (`KismetMathLibrary.RLerp` _returnvalue (`KismetMathLibrary.FindLookAtRotation` (+ (`KismetMathLibrary.GreaterGreater_VectorRotator` (-10.0 0.0 8.0) _returnvalue) (`SceneComponent.K2_GetComponentLocation` _flashlight)) (`.ImpactPoint` (`GameplayStatics.BreakHitResult` _hit))) 0.1 true) false false)
    (else
      (`SceneComponent.K2_SetWorldRotation` _flashlight (`KismetMathLibrary.RLerp` _returnvalue (struct) 0.1 true) false false))))

(fn `UserConstructionScript`)