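; Backup gun Blueprint holding nodes for firing effects and a flashlight toggle.
; FireTriggerEvent takes a hit result, spawns muzzle flash Niagara, places a randomly rotated, normal-aligned impact decal, and writes the impact point to a Material Parameter Collection for shader-driven glass destruction.
; Thumb Mouse Button 2 toggles the first found BP_Gun's flashlight, noted for moving to the FPC Blueprint.
; The pre-impact material check is an unconnected stub.
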(event `self.FireTriggerEvent`
  (params (Hit :type "HitResult Structure (by ref)") (ShotDirection :type "Vector Structure (by ref)") (AmmoType :type "AMMO_TYPES Enum" :default "Regular"))
  (bind (_bblockinghit _binitialoverlap _time _distance _location _impactpoint _normal _impactnormal) (`GameplayStatics.BreakHitResult` Hit))
  (bind _returnvalue (`KismetMathLibrary.RandomFloatInRange` 0.0 360.0))
  (bind (_x _y _z) (`KismetMathLibrary.BreakRotIntoAxes` (`KismetMathLibrary.Conv_VectorToRotator` _impactnormal)))
  (`|ExecutionSequence`
    (:`then_0`
      ;[1 1 1] Spawn Niagara System Attatched
      (`NiagaraFunctionLibrary.SpawnSystemAttached` (`self.MuzzleFlash`) (`self.SkeletalMesh`) "Muzzle" (100.0 0.0 5.0) (struct) "KeepRelativeOffset"))
    (:`then_1`
      ;[1 1 1] Spawn Decal At Hit Location
      (`GameplayStatics.SpawnDecalAtLocation` "/Game/Decals/HitDecals/D_Explosion_Wallbang.D_Explosion_Wallbang" (15.0 15.0 15.0) _impactpoint (`KismetMathLibrary.MakeRotationFromAxes` _x (`KismetMathLibrary.RotateAngleAxis` _y _returnvalue _x) (`KismetMathLibrary.RotateAngleAxis` _z _returnvalue _x)) (`KismetMathLibrary.RandomFloatInRange` 6.0 12.0)))
    (:`then_2`
      ;[1 1 1] Destroy Glass on Impact from Shader
      (`KismetMaterialLibrary.SetVectorParameterValue` "/Game/Materials/MaterialsVariableCollection/MPC_DestructibleShader.MPC_DestructibleShader" "ShaderHitLocation" (`KismetMathLibrary.Conv_VectorToLinearColor` (`.ImpactPoint` (`GameplayStatics.BreakHitResult` Hit)))))))

(event `Key|ThumbMouseButton2`
  (params (Key :type "Key Structure"))
  ;[1 1 1] Spotlight On / Off on F, MOVE TO FPC BP
  (:`Pressed`
    (bind _returnvalue (`GameplayStatics.GetActorOfClass` "/Game/Blueprints/Weapon/BP_Gun.BP_Gun_C"))
    (bind _flashlight (`/Game/Blueprints/Weapon/BP_Gun.Flashlight` _returnvalue))
    (if (`SceneComponent.bVisible` _flashlight)
      (`KismetSystemLibrary.PrintString` "Flashlight  ON, trying turning it off")
      (`SceneComponent.SetVisibility` _flashlight false false)
      (else
        (`KismetSystemLibrary.PrintString` "Flashlight OFF, Trying to turn it on")
        (`SceneComponent.SetVisibility` _flashlight true false)))))

(fn `UserConstructionScript`)