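; Gun Blueprint that provides the visual, audio and UI feedback for firing and reloading.
; Firing attaches a Niagara muzzle flash to the mesh's Muzzle socket and picks a sound by ammo type, attached for Regular and Bouncing, 2D for Explosive and Rapid.
; Reloading plays a 2D sound and shows a reloading widget until the completion event removes it.
; The fire event's hit result is unused.
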(event `self.ReloadCompletedEvent`
  (`Widget.RemoveFromParent` (stale `self.ReloadTriggerEvent` _returnvalue)))

(event `self.ReloadTriggerEvent`
  ;[1 1 1] Skjutljud
  (`GameplayStatics.SpawnSound2D` "/Game/Audio/SFX/Player/Weapon/Management/ReloadingSoundCue.ReloadingSoundCue" 1.0 1.0 0.0 null)
  (bind _returnvalue (`|CreateWidget` "/Game/UserInterface/W_Reloading.W_Reloading_C"))
  (`UserWidget.AddToViewport` _returnvalue 0))

(event `self.FireTriggerEvent`
  (params (Hit :type "HitResult Structure (by ref)") (ShotDirection :type "Vector Structure (by ref)") (AmmoType :type "AMMO_TYPES Enum" :default "Regular"))
  ;[1 1 1] Skjutljud
  ;[1 1 1] Spawn Niagara System Attatched
  (`NiagaraFunctionLibrary.SpawnSystemAttached` (`self.MuzzleFlash`) (`self.SkeletalMesh`) "Muzzle" (0.0 0.0 0.0) (struct) "KeepRelativeOffset")
  (if (`|EnumEquality` AmmoType "Regular")
    (`GameplayStatics.SpawnSoundAttached` "/Game/Audio/SFX/Player/Weapon/Default/ShootDefaultLayered.ShootDefaultLayered" (`self.SkeletalMesh`) "None" (0.0 0.0 0.0) (struct) "KeepRelativeOffset" false 1.0 1.0 0.0 null null :!label _label)
    (elif (`|EnumEquality` AmmoType "Bouncing")
      (goto _label)
      (elif (`|EnumEquality` AmmoType "Explosive")
        (`GameplayStatics.SpawnSound2D` "/Game/Audio/SFX/Player/Weapon/Explosive/S_Flare_Launcher_SPM.S_Flare_Launcher_SPM" 1.0 1.0 0.0 null)
        (elif (`|EnumEquality` AmmoType "Rapid")
          (`GameplayStatics.SpawnSound2D` "/Game/Audio/SFX/Player/Weapon/Default/ShootRapidLayered.ShootRapidLayered" 1.0 1.0 0.0 null))))))

(fn `UserConstructionScript`)