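; Explosive projectile Blueprint, named as a backup, that handles the visual impact effects when its hit event fires.
; HitTriggerEvent spawns a Niagara explosion at the impact point, then a short-lived wallbang decal aligned to the surface normal with random roll and lifespan.
; It also writes the impact point to a material parameter collection as ShaderHitLocation, so glass destruction is driven by shader.
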(event `self.HitTriggerEvent`
  (params (Hit :type "HitResult Structure (by ref)"))
  (bind (_bblockinghit _binitialoverlap _time _distance _location _impactpoint _normal _impactnormal) (`GameplayStatics.BreakHitResult` Hit))
  (bind _returnvalue (`KismetMathLibrary.RandomFloatInRange` 0.0 360.0))
  (bind (_x _y _z) (`KismetMathLibrary.BreakRotIntoAxes` (`KismetMathLibrary.Conv_VectorToRotator` _impactnormal)))
  (`|ExecutionSequence`
    (:`then_0`
      ;[1 1 1] Spawn System on Impact
      (`NiagaraFunctionLibrary.SpawnSystemAtLocation` "/Game/ParticleSystems/ImpactVFX/NS_Explosion.NS_Explosion" (`.ImpactPoint` (`GameplayStatics.BreakHitResult` Hit))))
    (:`then_1`
      ;[1 1 1] Spawn Decal At Hit Location
      (`GameplayStatics.SpawnDecalAtLocation` "/Game/Decals/D_Explosion_Wallbang.D_Explosion_Wallbang" (15.0 15.0 15.0) _impactpoint (`KismetMathLibrary.MakeRotationFromAxes` _x (`KismetMathLibrary.RotateAngleAxis` _y _returnvalue _x) (`KismetMathLibrary.RotateAngleAxis` _z _returnvalue _x)) (`KismetMathLibrary.RandomFloatInRange` 6.0 12.0)))
    (:`then_2`
      ;[1 1 1] Destroy Glass on Impact from Shader
      (`KismetMaterialLibrary.SetVectorParameterValue` "/Game/Materials/MaterialsVariableCollection/M_Destructible_Collection.M_Destructible_Collection" "ShaderHitLocation" (`KismetMathLibrary.Conv_VectorToLinearColor` (`.ImpactPoint` (`GameplayStatics.BreakHitResult` Hit)))))))

(fn `UserConstructionScript`)