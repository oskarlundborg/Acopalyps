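; Shotgun projectile that plays an attached sound on spawn and produces environmental impact effects when it hits.
; Its hit event does nothing for enemy AI characters and drones.
; Other hits spawn a Niagara impact effect and a normal-aligned decal with random size, roll and lifespan.
; The impact point is also written to a material parameter collection to drive shader-based glass destruction.
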(event `self.ReceiveBeginPlay`
  (`GameplayStatics.SpawnSoundAttached` "/Game/Audio/SFX/Player/Weapon/Sus/S_SusCue.S_SusCue" (`self.Mesh`) "None" (0.0 0.0 0.0) (struct) "KeepRelativeOffset" false 1.0 1.0 0.0 null null))

(event `self.HitTriggerEvent`
  (params (Hit :type "HitResult Structure (by ref)"))
  (bind (_bblockinghit _binitialoverlap _time _distance _location _impactpoint _normal _impactnormal _physmat _hitactor) (`GameplayStatics.BreakHitResult` Hit))
  (bind (_bblockinghit_2 _binitialoverlap_2 _time_2 _distance_2 _location_2 _impactpoint_2 _normal_2 _impactnormal_2) (`GameplayStatics.BreakHitResult` Hit))
  (bind _returnvalue (`KismetMathLibrary.RandomFloatInRange` 0.0 360.0))
  (bind _returnvalue_2 (`KismetMathLibrary.RandomFloatInRange` 2.0 4.5))
  (bind (_x _y _z) (`KismetMathLibrary.BreakRotIntoAxes` (`KismetMathLibrary.Conv_VectorToRotator` _impactnormal_2)))
  (cast `/Game/Blueprints/EnemyAI/BP_EnemyAICharacter` _hitactor
    (:`CastFailed`
      (cast `/Game/Blueprints/EnemyAI/BP_EnemyDroneBaseActor` _hitactor
        (:`CastFailed`
          (`|ExecutionSequence`
            (:`then_0`
              ;[1 1 1] Spawn System on Impact
              (`NiagaraFunctionLibrary.SpawnSystemAtLocation` "/Game/ParticleSystems/ImpactVFX/NS_Impact_Shotgun.NS_Impact_Shotgun" (`.ImpactPoint` (`GameplayStatics.BreakHitResult` Hit))))
            (:`then_1`
              ;[1 1 1] Spawn Decal At Hit Location
              (bind _returnvalue_3 (`GameplayStatics.SpawnDecalAtLocation` "/Game/Decals/HitDecals/D_Impact_Regular.D_Impact_Regular" (`KismetMathLibrary.MakeVector` _returnvalue_2 _returnvalue_2 _returnvalue_2) _impactpoint_2 (`KismetMathLibrary.MakeRotationFromAxes` _x (`KismetMathLibrary.RotateAngleAxis` _y _returnvalue _x) (`KismetMathLibrary.RotateAngleAxis` _z _returnvalue _x)) (`KismetMathLibrary.RandomFloatInRange` 6.0 12.0)))
              (`DecalComponent.SetFadeScreenSize` _returnvalue_3 0.001))
            (:`then_2`
              ;[1 1 1] Destroy Glass on Impact from Shader
              (`KismetMaterialLibrary.SetVectorParameterValue` "/Game/Materials/MaterialsVariableCollection/MPC_DestructibleShader.MPC_DestructibleShader" "ShaderHitLocation" (`KismetMathLibrary.Conv_VectorToLinearColor` (`.ImpactPoint` (`GameplayStatics.BreakHitResult` Hit)))))))))))

(fn `UserConstructionScript`)