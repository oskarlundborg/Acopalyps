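; Flare projectile that creates implosion effects, a decal and a light where it hits.
; The hit trigger event spawns a Niagara burst, a randomly sized and rotated fading decal, an attached sound, and, after a one-second delay, a BP_FlareLightActor.
; It also writes the impact point to a Material Parameter Collection so the destructible shader can break glass there.
; A separate Hit event destroys the trail component.
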(event `self.HitTriggerEvent`
  (params (Hit :type "HitResult Structure (by ref)"))
  (bind (_bblockinghit _binitialoverlap _time _distance _location _impactpoint _normal _impactnormal) (`GameplayStatics.BreakHitResult` Hit))
  (bind _returnvalue (`KismetMathLibrary.RandomFloatInRange` 0.0 360.0))
  (bind _returnvalue_2 (`KismetMathLibrary.RandomFloatInRange` 16.0 18.0))
  (bind (_x _y _z) (`KismetMathLibrary.BreakRotIntoAxes` (`KismetMathLibrary.Conv_VectorToRotator` _impactnormal)))
  (`|ExecutionSequence`
    (:`then_0`
      ;[1 1 1] Spawn System on Impact
      (`NiagaraFunctionLibrary.SpawnSystemAtLocation` "/Game/ParticleSystems/ImpactVFX/NS_ImplosionFlare.NS_ImplosionFlare" (`.ImpactPoint` (`GameplayStatics.BreakHitResult` Hit))))
    (:`then_1`
      ;[1 1 1] Spawn Decal At Hit Location
      (bind _returnvalue_3 (`GameplayStatics.SpawnDecalAtLocation` "/Game/Decals/HitDecals/D_Impact_Flare.D_Impact_Flare" (`KismetMathLibrary.MakeVector` _returnvalue_2 _returnvalue_2 _returnvalue_2) _impactpoint (`KismetMathLibrary.MakeRotationFromAxes` _x (`KismetMathLibrary.RotateAngleAxis` _y _returnvalue _x) (`KismetMathLibrary.RotateAngleAxis` _z _returnvalue _x)) (`KismetMathLibrary.RandomFloatInRange` 6.0 12.0)))
      (`DecalComponent.SetFadeScreenSize` _returnvalue_3 0.001))
    (:`then_2`
      ;[1 1 1] Destroy Glass on Impact from Shader
      (`KismetMaterialLibrary.SetVectorParameterValue` "/Game/Materials/MaterialsVariableCollection/MPC_DestructibleShader.MPC_DestructibleShader" "ShaderHitLocation" (`KismetMathLibrary.Conv_VectorToLinearColor` (`.ImpactPoint` (`GameplayStatics.BreakHitResult` Hit)))))
    (:`then_3`
      ;[1 1 1] Spawn Lightsource from BP_FlareLightActor (changes in Actor if needed)
      (`KismetSystemLibrary.Delay` 1.0)
      (`|SpawnActorFromClass` "/Game/Blueprints/Weapon/Projectiles/BP_FlareLightActor.BP_FlareLightActor_C" (`KismetMathLibrary.MakeTransform` (`.ImpactPoint` (`GameplayStatics.BreakHitResult` Hit))) "Undefined" "OverrideRootScale" null null))
    (:`then_4`
      (`/Engine/EditorBlueprintResources/StandardMacros.DoOnce` false :!label _label
        (:`Completed`
          (`GameplayStatics.SpawnSoundAttached` "/Game/Audio/SFX/Player/Weapon/Flare/LightImplosionCue.LightImplosionCue" (`self.Mesh`) "None" (0.0 0.0 0.0) (struct) "KeepRelativeOffset" false 1.0 1.0 0.0 null null)
          (goto _label :!via `Reset`))))))

(event `self.ReceiveHit`
  (params (MyComp :type "PrimitiveComponent Object Reference") (Other :type "Actor Object Reference") (OtherComp :type "PrimitiveComponent Object Reference") (bSelfMoved :type Boolean) (HitLocation :type "Vector Structure") (HitNormal :type "Vector Structure") (NormalImpulse :type "Vector Structure") (Hit :type "HitResult Structure (by ref)"))
  (`ActorComponent.K2_DestroyComponent` (`self.Trail`)))

(fn `UserConstructionScript`)