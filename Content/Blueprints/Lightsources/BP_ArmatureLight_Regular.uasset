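; BP_ArmatureLight_Regular is a light source actor that can be destroyed by damage.
; Explosive damage, detected by casting the damage type to BP_ExplosiveDamageType, flags it as destroyed and removes it immediately.
; A second sequence branch subtracts every hit from Health and does the same once Health drops below one.
; The construction script is empty, and destruction plays no animation.
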(event `self.ReceiveAnyDamage`
  (params (Damage :type "Float (single-precision)") (DamageType :type "DamageType Object Reference") (InstigatedBy :type "Controller Object Reference") (DamageCauser :type "Actor Object Reference"))
  ;[1 1 1] Destroy Lightsource // Add Animation in the end
  (`|ExecutionSequence`
    (:`then_0`
      (cast `/Game/Blueprints/Weapon/DamageType/BP_ExplosiveDamageType` DamageType)
      (set `self.IsDestroyed` true)
      (`self.K2_DestroyActor`))
    (:`then_1`
      (set `self.Health` (- (`self.Health`) Damage))
      (if (< (`self.Health`) 1.0)
        (set `self.IsDestroyed` true)
        (`self.K2_DestroyActor`)))))

(fn `UserConstructionScript`)