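; BP_Door is a trigger-driven door that opens and closes when the player character type, AcopalypsCharacter, enters its trigger boxes.
; OpenBox and CloseBox overlaps each fire once, playing their own sequence and a sliding sound at the door frame.
; When flagged IsExitDoor, closing also plays a 2D sound, currently named as a silent placeholder.
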(event `self.OpenBox.OnComponentBeginOverlap`
  (params (OverlappedComponent :type "PrimitiveComponent Object Reference") (OtherActor :type "Actor Object Reference") (OtherComp :type "PrimitiveComponent Object Reference") (OtherBodyIndex :type Integer) (bFromSweep :type Boolean) (SweepResult :type "HitResult Structure (by ref)"))
  (cast `AcopalypsCharacter` OtherActor)
  (`/Engine/EditorBlueprintResources/StandardMacros.DoOnce` false
    (:`Completed`
      (`ActorSequenceComponent.PlaySequence` (`self.OpenSequence`))
      (`GameplayStatics.SpawnSoundAtLocation` "/Game/Audio/SFX/Environment/ShowerDoorSlide_S08HS_815.ShowerDoorSlide_S08HS_815" (`SceneComponent.K2_GetComponentLocation` (`self.DoorFrame`)) (struct) 1.0 1.0 0.0 null null))))

(event `self.CloseBox.OnComponentBeginOverlap`
  (params (OverlappedComponent :type "PrimitiveComponent Object Reference") (OtherActor :type "Actor Object Reference") (OtherComp :type "PrimitiveComponent Object Reference") (OtherBodyIndex :type Integer) (bFromSweep :type Boolean) (SweepResult :type "HitResult Structure (by ref)"))
  (cast `AcopalypsCharacter` OtherActor)
  (`/Engine/EditorBlueprintResources/StandardMacros.DoOnce` false
    (:`Completed`
      (`ActorSequenceComponent.PlaySequence` (`self.CloseSequence`))
      (`GameplayStatics.SpawnSoundAtLocation` "/Game/Audio/SFX/Environment/ShowerDoorSlide_S08HS_814.ShowerDoorSlide_S08HS_814" (`SceneComponent.K2_GetComponentLocation` (`self.DoorFrame`)) (struct) 1.0 1.0 0.0 null null)
      (if (`self.IsExitDoor`)
        (`GameplayStatics.PlaySound2D` "/Game/Audio/OST/Silent_Placeholder.Silent_Placeholder" 1.0 1.0 0.0 null null)))))

(fn `UserConstructionScript`)