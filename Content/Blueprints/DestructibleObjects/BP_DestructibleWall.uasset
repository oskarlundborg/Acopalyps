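; BP_DestructibleWall is a box-shaped wall that gets holes carved into it where it is hit, using Geometry Script.
; Rebuilding the generated mesh appends a box of the configured Size and enables complex-as-simple collision.
; BeginPlay builds a small sphere-box mesh as the cutting tool, Projectile.
; The Destruction event converts the hit's impact point to local space and boolean-subtracts the scaled-up tool from the wall.
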(event `self.OnRebuildGeneratedMesh`
  (params (TargetMesh :type "DynamicMesh Object Reference"))
  (bind (_size_x _size_y _size_z) (`KismetMathLibrary.BreakVector` (`self.Size`)))
  ;[1 1 1] Making a BoxShape Destructible wall Object
  (bind _output_get (set `self.Target Mesh` TargetMesh))
  (`GeometryScriptLibrary_MeshPrimitiveFunctions.AppendBox` _output_get (struct) (struct) _size_x _size_y _size_z 0 0 0 "Base" null)
  (`DynamicMeshComponent.EnableComplexAsSimpleCollision` (`self.DynamicMeshComponent`)))

(event `self.ReceiveBeginPlay`
  ;[1 1 1] Making the projectile shape and promote Variable Name Projectile
  (bind _returnvalue (`self.AllocateComputeMesh`))
  (bind _returnvalue_2 (`GeometryScriptLibrary_MeshPrimitiveFunctions.AppendSphereBox` _returnvalue (struct) (struct) 10.0 6 6 6 "Center" null))
  (set `self.Projectile` _returnvalue_2))

(event `/Game/Blueprints/DestructibleObjects/BPI_Destructible.Destruction`
  (params (Hit :type "HitResult Structure") (Velocity :type "Vector Structure"))
  ;[1 1 1] Create new geometry via Boolean operation on mesh
  (`/Engine/EditorBlueprintResources/StandardMacros.IsValid` (`self.Projectile`)
    (:`Is Valid`
      (`GeometryScriptLibrary_MeshBooleanFunctions.ApplyMeshBoolean` (`self.Target Mesh`) (struct) (`self.Projectile`) (`KismetMathLibrary.MakeTransform` (`KismetMathLibrary.InverseTransformLocation` (`SceneComponent.K2_GetComponentToWorld` (`self.DynamicMeshComponent`)) (`.ImpactPoint` (`GameplayStatics.BreakHitResult` Hit))) (struct) (2.0 2.0 2.0)) "Subtract" (struct) null))))

(fn `UserConstructionScript`)